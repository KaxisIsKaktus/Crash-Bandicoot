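; Death trigger actor that handles overlaps by either failing Crash or pulling the player out of a bonus level.
; Any overlap first clears the bonus key count in Crash_GI.
; In a bonus level it opens the current progression level and moves the player pawn to the saved bonus checkpoint, without checking what overlapped.
; Otherwise it calls Lose on the overlapping Crash_BP.
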(event EventBeginPlay)

(event Collision|EventActorBeginOverlap
  (params (OtherActor :type Actor%20Object%20Reference))
  (bind _ascrash_gi (Utilities|Casting|CastToCrash_GI (Game|GetGameInstance)))
  (Variables|/Game/Game/Blueprints/Crash_GI.Crash_GI_C|SetBonus%20Keys _ascrash_gi 0)
  (if (Variables|/Game/Game/Blueprints/Crash_GI.Crash_GI_C|GetIn%20Bonus%20Level _ascrash_gi)
    (Game|OpenLevel(byName) (.levelname (Utilities|Array|Get(acopy) (Variables|/Game/Game/Blueprints/Crash_GI.Crash_GI_C|GetLevel%20Progression _ascrash_gi) (Variables|/Game/Game/Blueprints/Crash_GI.Crash_GI_C|GetCurrent%20Level%20Index _ascrash_gi))))
    (Transformation|SetActorLocation (Game|Player|GetPlayerPawn 0) (Variables|/Game/Game/Blueprints/Crash_GI.Crash_GI_C|GetBonus%20Checkpoint%20Location _ascrash_gi) false false)
    (else
      (bind _ascrash_bp (Utilities|Casting|CastToCrash_BP OtherActor))
      (Default|Lose _ascrash_bp))))

(event EventTick
  (params (DeltaSeconds :type Float%20%28single-precision%29)))

(fn ConstructionScript)