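; Fire trap platform hazard that cycles its flame on a timer and makes the player lose on contact.
; BeginPlay runs an endless Delay loop: off, a brief warning-length puff, off again, then a full-scale burst before shrinking the particle system and restarting.
; Overlap on the ParticleSystem component casts the other actor to Crash_BP and calls Lose, without checking whether the flame is active.
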(event OnComponentBeginOverlap(ParticleSystem)
  (params (OverlappedComponent :type Primitive%20Component%20Object%20Reference) (OtherActor :type Actor%20Object%20Reference) (OtherComp :type Primitive%20Component%20Object%20Reference) (OtherBodyIndex :type Integer) (bFromSweep :type Boolean) (SweepResult :type Hit%20Result%20Structure%20%28by%20ref%29))
  (bind _ascrash_bp (Utilities|Casting|CastToCrash_BP OtherActor))
  (Default|Lose _ascrash_bp))

(event EventBeginPlay
  (Components|Activation|Deactivate (Variables|Default|GetParticleSystem) :!label _label)
  (Utilities|FlowControl|Delay 2.0)
  (Components|Activation|Activate (Variables|Default|GetParticleSystem) false)
  (Utilities|FlowControl|Delay 0.2)
  (Components|Activation|Deactivate (Variables|Default|GetParticleSystem))
  (Utilities|FlowControl|Delay 1.0)
  (Components|Activation|Activate (Variables|Default|GetParticleSystem) false)
  (Transformation|SetWorldScale3D (Variables|Default|GetParticleSystem) "1.000000,1.000000,1.000000")
  (Utilities|FlowControl|Delay 1.0)
  (Transformation|SetWorldScale3D (Variables|Default|GetParticleSystem) "0.100000,0.100000,0.100000")
  (goto _label))

(fn ConstructionScript)