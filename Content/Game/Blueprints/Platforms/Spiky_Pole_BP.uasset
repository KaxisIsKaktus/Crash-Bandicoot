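; Spiky pole Blueprint that moves back and forth endlessly between its placed location and an EndPoint component's location.
; BeginPlay caches both world positions, then starts the Up event.
; Up and Down each play their own Timeline to lerp the actor's location without sweeping, then call each other after a delay, pausing longer at the start than at the end.
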(event Custom|Up
  (bind _float (Timeline|Timeline PlayFromStart)
    (:Update
      (Transformation|SetActorLocation (Math|Vector|Lerp(Vector) (Variables|Default|GetStart) (Variables|Default|GetFinish) _float) false false))
    (:Finished
      (Utilities|FlowControl|Delay 1.0)
      (CallFunction|Down))))

(event Custom|Down
  (bind _float (Timeline|Timeline_0 PlayFromStart)
    (:Update
      (Transformation|SetActorLocation (Math|Vector|Lerp(Vector) (Variables|Default|GetFinish) (Variables|Default|GetStart) _float) false false))
    (:Finished
      (Utilities|FlowControl|Delay 3.0)
      (CallFunction|Up))))

(event EventBeginPlay
  (Variables|Default|SetFinish (Transformation|GetWorldLocation (Variables|Default|GetEnd%20Point)))
  (Variables|Default|SetStart (Transformation|GetActorLocation))
  (CallFunction|Up))

(fn ConstructionScript)