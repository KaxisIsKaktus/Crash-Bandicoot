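; Level camera actor that follows the player along a CameraPath spline.
; Each tick it moves the SpringArm to the spline point closest to the player, plus an Offset and a lookahead along the path tangent.
; The lookahead is scaled by the dot product of tangent and player forward, so it shifts with facing.
; Arm yaw follows the spline, with a Sideways flag choosing a level side view or a pitched-down along-path view.
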(event EventTick
  (params (DeltaSeconds :type Float%20%28single-precision%29))
  (bind _returnvalue (Game|Player|GetPlayerPawn 0))
  (bind _camera_path (Variables|Default|GetCamera%20Path))
  (bind _sideways (Variables|Default|GetSideways))
  (bind _returnvalue_2 (Transformation|GetActorLocation _returnvalue))
  (bind _returnvalue_3 (Spline|FindDirectionClosesttoWorldLocation _camera_path _returnvalue_2 "World"))
  (Transformation|SetWorldLocation (Variables|Default|GetSpringArm) (+ (Spline|FindLocationClosesttoWorldLocation _camera_path _returnvalue_2 "World") (* _returnvalue_3 (Variables|Default|GetLookahead%20Distance) (Math|Vector|DotProduct _returnvalue_3 (Transformation|GetActorForwardVector (Game|Player|GetPlayerPawn 0)))) (Variables|Default|GetOffset)) false false)
  (Transformation|SetWorldRotation (Variables|Default|GetSpringArm) (Math|Rotator|MakeRotator 0.0 (Math|Float|SelectFloat 0.0 -4e+01 _sideways) (+ (Math|Float|SelectFloat -9e+01 0.0 _sideways) (.yaw (Class|SplineComponent|FindRotationClosesttoWorldLocation (Variables|Default|GetCamera%20Path) _returnvalue_2 "World")))) false false))

(fn ConstructionScript)