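; Turtle enemy that patrols between its start position and an EndPoint and can be flipped by Crash_BP to serve as a bounce pad.
; A Timeline lerps the location back and forth, with play rate scaled by Speed over distance.
; TopTrigger bounces Crash, stops the patrol and rolls the turtle over on a second Timeline.
; BottomTrigger launches Crash higher, while HurtTrigger calls Lose on Crash.
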(event OnComponentBeginOverlap(HurtTrigger)
  (params (OverlappedComponent :type Primitive%20Component%20Object%20Reference) (OtherActor :type Actor%20Object%20Reference) (OtherComp :type Primitive%20Component%20Object%20Reference) (OtherBodyIndex :type Integer) (bFromSweep :type Boolean) (SweepResult :type Hit%20Result%20Structure%20%28by%20ref%29))
  (bind _ascrash_bp (Utilities|Casting|CastToCrash_BP OtherActor))
  (Default|Lose _ascrash_bp))

(event OnComponentBeginOverlap(TopTrigger)
  (params (OverlappedComponent :type Primitive%20Component%20Object%20Reference) (OtherActor :type Actor%20Object%20Reference) (OtherComp :type Primitive%20Component%20Object%20Reference) (OtherBodyIndex :type Integer) (bFromSweep :type Boolean) (SweepResult :type Hit%20Result%20Structure%20%28by%20ref%29))
  ;[1 1 1] Turtle flipping
  (bind _ascrash_bp (Utilities|Casting|CastToCrash_BP OtherActor))
  (Character|LaunchCharacter _ascrash_bp "0.000000,0.000000,800.000000" false true)
  (Utilities|FlowControl|Sequence
    (:then_0
      ;[1 1 1] Turtle movement
      (bind (_direction _float) (Timeline|Timeline Stop)
        (:Update
          (Transformation|SetActorLocation (Math|Vector|Lerp(Vector) (Variables|Default|GetStart) (Variables|Default|GetFinish) _float) false false))
        (:Finished
          (switch Utilities|FlowControl|Switch|SwitchonETimelineDirection _direction
            (:Forward
              (Timeline|Timeline Reverse))
            (:Backward
              (Timeline|Timeline PlayFromStart))))))
    (:then_1
      (bind _float_2 (Timeline|Flip%20turtle%20timeline Play)
        (:Update
          (Transformation|SetActorRotation (Math|Rotator|MakeRotator (Math|Float|Lerp 0.0 1.8e+02 _float_2) 0.0 0.0)))))))

(event OnComponentBeginOverlap(BottomTrigger)
  (params (OverlappedComponent :type Primitive%20Component%20Object%20Reference) (OtherActor :type Actor%20Object%20Reference) (OtherComp :type Primitive%20Component%20Object%20Reference) (OtherBodyIndex :type Integer) (bFromSweep :type Boolean) (SweepResult :type Hit%20Result%20Structure%20%28by%20ref%29))
  ;[1 1 1] Jumping on the turtle
  (bind _ascrash_bp (Utilities|Casting|CastToCrash_BP OtherActor))
  (Character|LaunchCharacter _ascrash_bp "0.000000,0.000000,1000.000000" false true))

(event EventBeginPlay
  ;[1 1 1] Turtle movement
  (Variables|Default|SetFinish (Transformation|GetWorldLocation (Variables|Default|GetEnd%20Point)))
  (Variables|Default|SetStart (Transformation|GetActorLocation))
  (Components|Timeline|SetPlayRate (Variables|Default|GetTimeline) (/ (Variables|Default|GetSpeed) (Math|Vector|VectorLength (- (Variables|Default|GetFinish) (Variables|Default|GetStart)))))
  (bind (_direction _float) (Timeline|Timeline Play)
    (:Update
      (Transformation|SetActorLocation (Math|Vector|Lerp(Vector) (Variables|Default|GetStart) (Variables|Default|GetFinish) _float) false false))
    (:Finished
      (switch Utilities|FlowControl|Switch|SwitchonETimelineDirection _direction
        (:Forward
          (Timeline|Timeline Reverse))
        (:Backward
          (Timeline|Timeline PlayFromStart))))))

(fn ConstructionScript
  (|CallParentFunction))