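; Teleporter actor that moves the player to the next level, or into and out of a bonus level.
; Overlapping its sphere advances the Crash_GI level progression, ending at the main menu; bonus teleporters require three keys and get their own material.
; Crash_GI stores the bonus state and teleporter location across level loads.
; On BeginPlay after a bonus return, an active teleporter disables its collision and restores the player there.
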(event OnComponentBeginOverlap(Sphere)
  (params (OverlappedComponent :type Primitive%20Component%20Object%20Reference) (OtherActor :type Actor%20Object%20Reference) (OtherComp :type Primitive%20Component%20Object%20Reference) (OtherBodyIndex :type Integer) (bFromSweep :type Boolean) (SweepResult :type Hit%20Result%20Structure%20%28by%20ref%29))
  ;[1 1 1] Teleporting system
  (if (Variables|Default|GetBonus)
    (bind _ascrash_gi (Utilities|Casting|CastToCrash_GI (Game|GetGameInstance)))
    (if (== (Variables|/Game/Game/Blueprints/Crash_GI.Crash_GI_C|GetBonus%20Keys _ascrash_gi) 3)
      (CallFunction|LoadBonusLevel))
    (else
      (CallFunction|LoadLevel))))

(event Custom|Load%20Level
  (Input|DisableInput (Game|Player|GetPlayerPawn 0) (Game|GetPlayerController 0))
  (Utilities|FlowControl|Delay 1.0)
  (bind _ascrash_gi (Utilities|Casting|CastToCrash_GI (Game|GetGameInstance)))
  (bind _result (Math|Integer|IncrementInt (Variables|/Game/Game/Blueprints/Crash_GI.Crash_GI_C|GetCurrent%20Level%20Index _ascrash_gi))
    (:%20%20
      (if (not (< _result (Utilities|Array|Length (Variables|/Game/Game/Blueprints/Crash_GI.Crash_GI_C|GetLevel%20Progression _ascrash_gi))))
        (Game|OpenLevel(byObjectReference) "/Game/Game/Maps/MainMenu.MainMenu")
        (else
          (Transformation|SetActorTransform (Game|Player|GetPlayerPawn 0) (Utilities|Array|Get(acopy) (Variables|/Game/Game/Blueprints/Crash_GI.Crash_GI_C|GetLevel%20Start%20Location _ascrash_gi) _result))
          (Game|OpenLevel(byName) (.levelname (Utilities|Array|Get(acopy) (Variables|/Game/Game/Blueprints/Crash_GI.Crash_GI_C|GetLevel%20Progression _ascrash_gi) _result))))))))

(event Custom|Load%20Bonus%20Level
  (Input|DisableInput (Game|Player|GetPlayerPawn 0) (Game|GetPlayerController 0))
  (Utilities|FlowControl|Delay 1.0)
  (bind _ascrash_gi (Utilities|Casting|CastToCrash_GI (Game|GetGameInstance)))
  (if (Variables|/Game/Game/Blueprints/Crash_GI.Crash_GI_C|GetIn%20Bonus%20Level _ascrash_gi)
    (Variables|/Game/Game/Blueprints/Crash_GI.Crash_GI_C|SetIn%20Bonus%20Level _ascrash_gi false)
    (Game|OpenLevel(byName) (.LevelName (Utilities|Struct|BreakLevel_Name_STRUCT (Utilities|Array|Get(acopy) (Variables|/Game/Game/Blueprints/Crash_GI.Crash_GI_C|GetLevel%20Progression _ascrash_gi) (Variables|/Game/Game/Blueprints/Crash_GI.Crash_GI_C|GetCurrent%20Level%20Index _ascrash_gi)))))
    (Transformation|SetActorLocation (Game|Player|GetPlayerPawn 0) (Variables|/Game/Game/Blueprints/Crash_GI.Crash_GI_C|GetBonus%20Checkpoint%20Location _ascrash_gi) false false)
    (Variables|/Game/Game/Blueprints/Crash_GI.Crash_GI_C|SetBonus%20Keys _ascrash_gi 0)
    (else
      (Variables|/Game/Game/Blueprints/Crash_GI.Crash_GI_C|SetIn%20Bonus%20Level _ascrash_gi true)
      (Variables|/Game/Game/Blueprints/Crash_GI.Crash_GI_C|SetBonus%20Checkpoint%20Activated _ascrash_gi true)
      (Variables|/Game/Game/Blueprints/Crash_GI.Crash_GI_C|SetBonus%20Checkpoint%20Location _ascrash_gi (Transformation|GetActorLocation))
      (Game|OpenLevel(byName) (.BonusLevelName (Utilities|Struct|BreakLevel_Name_STRUCT (Utilities|Array|Get(acopy) (Variables|/Game/Game/Blueprints/Crash_GI.Crash_GI_C|GetLevel%20Progression _ascrash_gi) (Variables|/Game/Game/Blueprints/Crash_GI.Crash_GI_C|GetCurrent%20Level%20Index _ascrash_gi))))))))

(event EventBeginPlay
  (bind _ascrash_gi (Utilities|Casting|CastToCrash_GI (Game|GetGameInstance)))
  (if (Math|Boolean|ANDBoolean (Variables|/Game/Game/Blueprints/Crash_GI.Crash_GI_C|GetBonus%20Checkpoint%20Activated _ascrash_gi) (not (Variables|/Game/Game/Blueprints/Crash_GI.Crash_GI_C|GetIn%20Bonus%20Level _ascrash_gi)) (Variables|Default|GetActive))
    (Collision|SetCollisionEnabled (Variables|Default|GetSphere) "NoCollision")
    (Transformation|SetActorLocation (Game|Player|GetPlayerPawn 0) (Variables|/Game/Game/Blueprints/Crash_GI.Crash_GI_C|GetBonus%20Checkpoint%20Location _ascrash_gi) false false)
    (Variables|/Game/Game/Blueprints/Crash_GI.Crash_GI_C|SetBonus%20Checkpoint%20Activated _ascrash_gi false)))

(fn ConstructionScript
  (Rendering|Material|SetMaterial (Variables|Default|GetTeleport) 0 (select (Variables|Default|GetBonus) "/Game/StarterContent/Materials/M_Tech_Hex_Tile.M_Tech_Hex_Tile" "/Game/StarterContent/Materials/M_Tech_Hex_Tile_Pulse.M_Tech_Hex_Tile_Pulse")))