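; Base collectible that Crash_BP picks up on overlap, running an empty ActionOnCollect hook for child classes, then destroying itself.
; Timelines drive the mesh's relative Z through an optional spawn animation, followed by an idle animation.
; A Gate blocks pickup until the spawn animation finishes, or opens at BeginPlay when ImmediateCollect is set or the spawn animation is disabled.
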(event OnComponentBeginOverlap(StaticMesh)
  (params (OverlappedComponent :type Primitive%20Component%20Object%20Reference) (OtherActor :type Actor%20Object%20Reference) (OtherComp :type Primitive%20Component%20Object%20Reference) (OtherBodyIndex :type Integer) (bFromSweep :type Boolean) (SweepResult :type Hit%20Result%20Structure%20%28by%20ref%29))
  (Utilities|Casting|CastToCrash_BP OtherActor)
  (Utilities|FlowControl|Gate true
    (:Exit
      (CallFunction|ActiononCollect)
      (Actor|DestroyActor))))

(event Custom|Start%20Idle%20Animation
  ;[1 1 1] Idle Animation
  (bind _z_coord (Timeline|Idle%20Timeline PlayFromStart)
    (:Update
      (Transformation|SetRelativeLocation (Variables|Default|GetStatic%20Mesh) (Math|Vector|MakeVector 0.0 0.0 _z_coord) false false))))

(event Custom|Action%20on%20Collect)

(event EventBeginPlay
  (if (Variables|Default|GetSpawn%20Animation%20Enabled)
    (if (Variables|Default|GetImmediate%20Collect)
      (Utilities|FlowControl|Sequence
        (:then_0
          (Utilities|FlowControl|Gate true) ; enters at Open
        )
        (:then_1
          (bind _z_coord (Timeline|Spawn%20Timeline PlayFromStart)
            (:Update
              (Transformation|SetRelativeLocation (Variables|Default|GetStatic%20Mesh) (Math|Vector|MakeVector 0.0 0.0 _z_coord) false false))
            (:Finished
              (CallFunction|StartIdleAnimation)
              (Utilities|FlowControl|Gate true) ; enters at Open
            ))))
      (else
        (Timeline|Spawn%20Timeline PlayFromStart)))
    (else
      (CallFunction|StartIdleAnimation)
      (Utilities|FlowControl|Gate true) ; enters at Open
    )))

(event Game|Damage|EventAnyDamage
  (params (Damage :type Float%20%28single-precision%29) (DamageType :type Damage%20Type%20Object%20Reference) (InstigatedBy :type Controller%20Object%20Reference) (DamageCauser :type Actor%20Object%20Reference)))

(fn ConstructionScript)