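; Collectible Blueprint for a bonus key pickup, built on a parent collectible class.
; On collect, it increments the BonusKeys count on the Crash game instance and prints the new total to the screen.
; BeginPlay and the construction script only call their parent versions.
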(event EventBeginPlay
  (|CallParentFunction))

(event EventActiononCollect
  (bind _ascrash_gi (Utilities|Casting|CastToCrash_GI (Game|GetGameInstance)))
  (bind _result (Math|Integer|IncrementInt (Variables|/Game/Game/Blueprints/Crash_GI.Crash_GI_C|GetBonus%20Keys _ascrash_gi))
    (:%20%20
      (Development|PrintString (Utilities|String|Append "Bonus Keys: " (Utilities|String|ToString(Integer) _result))))))

(fn ConstructionScript
  (|CallParentFunction))