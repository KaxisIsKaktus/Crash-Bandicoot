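; Spline path Blueprint that moves a referenced Actor once along its spline when play begins.
; The construction script snaps the Actor to the first point, and a Timeline, rate-scaled by TimelineLenght, lerps distance to the last point.
; Each movement update restarts TimelineRotation, whose Finished output sets rotation from the spline's start tangent plus the timeline's pitch offset, rather than following the current tangent.
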(event Custom|Play%20timeline
  (bind _actor (Variables|Default|GetActor))
  (bind _spline (Variables|Default|GetSpline))
  (bind _spline_2 (Variables|Default|GetSpline))
  (bind _returnvalue (Spline|GetTangentatDistanceAlongSpline _spline_2 0.0 "World"))
  (bind _returnvalue_2 (Math|Conversions|RotationFromXVector _returnvalue))
  ;[1 1 1] Movement
  (bind _float (Timeline|Timeline PlayFromStart)
    (:Update
      (Transformation|SetActorLocation _actor (Spline|GetLocationatDistanceAlongSpline _spline_2 (Math|Float|Lerp 0.0 (Spline|GetDistanceAlongSplineatSplinePoint _spline (- (Spline|GetNumberOfSplinePoints _spline) 1)) _float) "World") false false)
      (bind _float_2 (Timeline|Timeline%20Rotation PlayFromStart)
        (:Finished
          (Transformation|SetActorRotation _actor (Math|Rotator|MakeRotator (.roll _returnvalue_2) (+ _float_2 (.pitch _returnvalue_2)) (.yaw _returnvalue_2))))))))

(event EventBeginPlay
  ;[1 1 1] Event Begin Play
  (Components|Timeline|SetPlayRate (Variables|Default|GetTimeline) (/ 1.0 (Variables|Default|GetTimeline%20Lenght)))
  (CallFunction|PlayTimeline))

(fn ConstructionScript
  (Transformation|SetActorLocation (Variables|Default|GetActor) (Spline|GetLocationatSplinePoint (Variables|Default|GetSpline) 0 "World") false false))