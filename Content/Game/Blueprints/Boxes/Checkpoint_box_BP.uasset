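; Checkpoint crate that saves a checkpoint the first time it is broken by a bounce or damage.
; BounceAction and AnyDamage both call Break, which runs once, disables bouncing and writes the active flag and CheckpointMarker's world location to Crash_GI.
; A timeline then squashes the mesh into a wide, flat shape by lerping its scale and height.
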(event EventBeginPlay
  (|CallParentFunction))

(event Collision|EventActorBeginOverlap
  (params (OtherActor :type Actor%20Object%20Reference))
  (|CallParentFunction OtherActor))

(event EventTick
  (params (DeltaSeconds :type Float%20%28single-precision%29))
  (|CallParentFunction DeltaSeconds))

(event Game|Damage|EventAnyDamage
  (params (Damage :type Float%20%28single-precision%29) (DamageType :type Damage%20Type%20Object%20Reference) (InstigatedBy :type Controller%20Object%20Reference) (DamageCauser :type Actor%20Object%20Reference))
  (CallFunction|Break))

(event EventBreak
  (Utilities|FlowControl|DoOnce false
    (:Completed
      (Variables|Default|SetBounce%20Enabled false)
      (bind _ascrash_gi (Utilities|Casting|CastToCrash_GI (Game|GetGameInstance)))
      (Variables|/Game/Game/Blueprints/Crash_GI.Crash_GI_C|SetCheckpoint%20Activated _ascrash_gi true)
      (Variables|/Game/Game/Blueprints/Crash_GI.Crash_GI_C|SetCheckpoint%20Location _ascrash_gi (Transformation|GetWorldLocation (Variables|Default|GetCheckpoint%20Marker)))
      (bind _float (Timeline|Timeline_0 Play)
        (:Update
          (Transformation|SetWorldScale3D (Variables|Default|GetStaticMesh) (Math|Vector|Lerp(Vector) "1.000000,1.000000,1.000000" "2.000000,2.000000,0.100000" _float))
          (Transformation|SetRelativeLocation (Variables|Default|GetStaticMesh) (Math|Vector|Lerp(Vector) "0.000000,0.000000,50.000000" "0.000000,0.000000,5.000000" _float) false false))))))

(event EventBounceAction
  (CallFunction|Break))

(fn ConstructionScript
  (|CallParentFunction))