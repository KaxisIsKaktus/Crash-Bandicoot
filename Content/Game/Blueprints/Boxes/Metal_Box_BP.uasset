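; Metal box Blueprint that makes Crash lose when he touches its underside and can play a wobble animation.
; An overlap on BottomSurface casts the other actor to Crash_BP and calls its Lose function.
; BounceAnimation runs a timeline that tilts the static mesh's world roll, keeping pitch and yaw, then reverses to return it to upright.
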(event OnComponentBeginOverlap(BottomSurface)
  (params (OverlappedComponent :type Primitive%20Component%20Object%20Reference) (OtherActor :type Actor%20Object%20Reference) (OtherComp :type Primitive%20Component%20Object%20Reference) (OtherBodyIndex :type Integer) (bFromSweep :type Boolean) (SweepResult :type Hit%20Result%20Structure%20%28by%20ref%29))
  (bind _ascrash_bp (Utilities|Casting|CastToCrash_BP OtherActor))
  (Default|Lose _ascrash_bp))

(event EventBeginPlay
  (|CallParentFunction) ; This node is disabled and will not be called.\nDrag off pins to build functionality.
)

(event Collision|EventActorBeginOverlap
  (params (OtherActor :type Actor%20Object%20Reference))
  (|CallParentFunction OtherActor) ; This node is disabled and will not be called.\nDrag off pins to build functionality.
)

(event EventTick
  (params (DeltaSeconds :type Float%20%28single-precision%29))
  (|CallParentFunction DeltaSeconds) ; This node is disabled and will not be called.\nDrag off pins to build functionality.
)

(event EventBounceAnimation
  (bind _staticmesh (Variables|Default|GetStaticMesh))
  (bind _returnvalue (Transformation|GetWorldRotation _staticmesh))
  (bind (_direction _float) (Timeline|Timeline PlayFromStart)
    (:Update
      (Transformation|SetWorldRotation _staticmesh (Math|Rotator|MakeRotator (Math|Float|Lerp 0.0 15.0 _float) (.pitch _returnvalue) (.yaw _returnvalue)) false false))
    (:Finished
      (switch Utilities|FlowControl|Switch|SwitchonETimelineDirection _direction
        (:Forward
          (Timeline|Timeline ReverseFromEnd))))))

(fn ConstructionScript
  (|CallParentFunction))