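; Wooden breakable box that drops one collectible of a configured type: fruit, Aku Aku, extra life or bonus level key.
; Any damage, or a bounce when the box has no arrow, spawns the collectible through a DoOnce and calls Break.
; A separate bounce animation event squashes and stretches the mesh with a timeline that reverses itself.
; The construction script sets the box's text symbol from the collectible type and fruit count.
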(event EventBeginPlay
  (|CallParentFunction) ; This node is disabled and will not be called.\nDrag off pins to build functionality.
)

(event Collision|EventActorBeginOverlap
  (params (OtherActor :type Actor%20Object%20Reference))
  (|CallParentFunction OtherActor) ; This node is disabled and will not be called.\nDrag off pins to build functionality.
)

(event EventTick
  (params (DeltaSeconds :type Float%20%28single-precision%29))
  (|CallParentFunction DeltaSeconds) ; This node is disabled and will not be called.\nDrag off pins to build functionality.
)

(event Game|Damage|EventAnyDamage
  (params (Damage :type Float%20%28single-precision%29) (DamageType :type Damage%20Type%20Object%20Reference) (InstigatedBy :type Controller%20Object%20Reference) (DamageCauser :type Actor%20Object%20Reference))
  ;[1 1 1] Any Damage
  (CallFunction|SpawnCollectible)
  (CallFunction|Break))

(event EventBounceAnimation
  ;[1 1 1] Bounce animation of the box
  (bind (_direction _float) (Timeline|Timeline PlayFromStart)
    (:Update
      (Transformation|SetWorldScale3D (Variables|Default|GetStaticMesh) (Math|Vector|MakeVector (Math|Float|Lerp 1.0 1.5 _float) (Math|Float|Lerp 1.0 1.5 _float) (Math|Float|Lerp 1.0 0.5 _float))))
    (:Finished
      (switch Utilities|FlowControl|Switch|SwitchonETimelineDirection _direction
        (:Forward
          (Timeline|Timeline ReverseFromEnd))))))

(event EventBounceAction
  (if (not (Variables|Default|GetHas%20Arrow))
    (CallFunction|SpawnCollectible)
    (CallFunction|Break)))

(event EventSpawnCollectible
  (Utilities|FlowControl|DoOnce false
    (:Completed
      (switch Utilities|FlowControl|Switch|SwitchonCollectible_Types_ENUM (Variables|Default|GetCollectible%20type)
        (:NewEnumerator0
          (Game|SpawnActorfromClass "/Game/Game/Blueprints/Collectibles/Collectible_Fruit_BP.Collectible_Fruit_BP_C" (Transformation|GetWorldTransform (Variables|Default|GetStaticMesh)) "Undefined" "MultiplyWithRoot" 0 true false 0))
        (:NewEnumerator1
          (Game|SpawnActorfromClass "/Game/Game/Blueprints/Collectibles/Collectible_Aku_Aku_BP.Collectible_Aku_Aku_BP_C" (Transformation|GetWorldTransform (Variables|Default|GetStaticMesh)) "Undefined" "MultiplyWithRoot" 0 false false 0))
        (:NewEnumerator2
          (Game|SpawnActorfromClass "/Game/Game/Blueprints/Collectibles/Collectible_ExtraLife_BP.Collectible_ExtraLife_BP_C" (Transformation|GetWorldTransform (Variables|Default|GetStaticMesh)) "Undefined" "MultiplyWithRoot" 0 false false 0))
        (:NewEnumerator3
          (Game|SpawnActorfromClass "/Game/Game/Blueprints/Collectibles/Collectible_Bonus_Key_BP.Collectible_Bonus_Key_BP_C" (Transformation|GetWorldTransform (Variables|Default|GetStaticMesh)) "Undefined" "MultiplyWithRoot" 0 false false 0))))))

(fn ConstructionScript
  (CallFunction|InitializeBox)
  (|CallParentFunction))

(fn InitializeBox
  (Variables|Default|SetBox%20Text (Utilities|Select :Index (Variables|Default|GetCollectible%20type) :NewEnumerator0 (select (> (Variables|Default|GetNumber%20of%20fruits) 1) "?" "") :NewEnumerator1 "*" :NewEnumerator2 "+" :NewEnumerator3 ";)")))