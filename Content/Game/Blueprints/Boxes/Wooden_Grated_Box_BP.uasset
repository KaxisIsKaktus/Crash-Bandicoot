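; Wooden grated box that hands out fruit collectibles when bounced on and breaks after a set number of bounces.
; Each bounce action decrements the bounce counter, spawns an animated, immediately collected fruit at the mesh transform, and calls Break when the count reaches zero.
; Any damage calls Break directly, without spawning fruit in this graph; Break's logic is defined outside this file.
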(event EventBeginPlay
  (|CallParentFunction) ; This node is disabled and will not be called.\nDrag off pins to build functionality.
)

(event Collision|EventActorBeginOverlap
  (params (OtherActor :type Actor%20Object%20Reference))
  (|CallParentFunction OtherActor) ; This node is disabled and will not be called.\nDrag off pins to build functionality.
)

(event EventTick
  (params (DeltaSeconds :type Float%20%28single-precision%29))
  (|CallParentFunction DeltaSeconds) ; This node is disabled and will not be called.\nDrag off pins to build functionality.
)

(event Game|Damage|EventAnyDamage
  (params (Damage :type Float%20%28single-precision%29) (DamageType :type Damage%20Type%20Object%20Reference) (InstigatedBy :type Controller%20Object%20Reference) (DamageCauser :type Actor%20Object%20Reference))
  (CallFunction|Break))

(event EventSpawnCollectible
  (Game|SpawnActorfromClass "/Game/Game/Blueprints/Collectibles/Collectible_Fruit_BP.Collectible_Fruit_BP_C" (Transformation|GetWorldTransform (Variables|Default|GetStaticMesh)) "Undefined" "MultiplyWithRoot" 0 true true 0))

(event EventBounceAction
  (bind _result (Math|Integer|DecrementInt (Variables|Default|GetNumber%20of%20Bounces))
    (:%20%20
      (CallFunction|SpawnCollectible)
      (if (== _result 0)
        (CallFunction|Break)))))

(fn ConstructionScript
  (|CallParentFunction))