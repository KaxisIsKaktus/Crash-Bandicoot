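; Transparent placeholder box that turns into a real box when an Activator fires its ActivateBoxes event.
; On BeginPlay it binds Activate to that event.
; Activate spawns the configured ReplacementBox 50 cm below the placeholder with the same rotation and scale, then destroys itself.
; When the replacement is a Wooden_Regular_Box_BP, it also passes along its CollectibleType.
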(event Custom|Activate
  (bind _returnvalue (Transformation|GetActorTransform))
  (bind (_location _rotation _scale) (Math|Transform|BreakTransform _returnvalue))
  (bind (_x _y _z) (Math|Vector|BreakVector _location))
  (Variables|Default|SetCorrect%20Location (Math|Transform|MakeTransform (Math|Vector|MakeVector _x _y (- _z 5e+01)) _rotation _scale))
  (if (== (Variables|Default|GetReplacement%20Box) "/Game/Game/Blueprints/Boxes/Wooden_Regular_Box_BP.Wooden_Regular_Box_BP_C")
    (Game|SpawnActorfromClass "/Game/Game/Blueprints/Boxes/Wooden_Regular_Box_BP.Wooden_Regular_Box_BP_C" (Variables|Default|GetCorrect%20Location) "Undefined" "MultiplyWithRoot" 0 (Variables|Default|GetCollectible%20type) 0)
    (Actor|DestroyActor)
    (else
      (Game|SpawnActorfromClass (Variables|Default|GetReplacement%20Box) (Variables|Default|GetCorrect%20Location) "Undefined" "MultiplyWithRoot" 0 0)
      (Actor|DestroyActor))))

(event EventBeginPlay
  (EventDispatchers|BindEventtoActivateBoxes (Variables|Default|GetActivator) (delegate Custom|Activate)))

(event Collision|EventActorBeginOverlap
  (params (OtherActor :type Actor%20Object%20Reference)))

(event EventTick
  (params (DeltaSeconds :type Float%20%28single-precision%29)))

(fn ConstructionScript)