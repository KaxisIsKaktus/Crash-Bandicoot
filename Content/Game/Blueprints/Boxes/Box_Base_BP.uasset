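; Base crate for a Crash-style game that bounces the player from its top, with construction-time arrow visibility and text labels.
; Top overlaps, when bounce or arrow is enabled, launch Crash along the surface's up vector, stronger with arrows; arrow crates also pop other boxes upward.
; Top bounces and bottom hits by Crash call empty action/animation hooks.
; Ending a bottom overlap enables physics with an upward kick on physics-enabled boxes.
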(event OnComponentBeginOverlap(TopSurface)
  (params (OverlappedComponent :type Primitive%20Component%20Object%20Reference) (OtherActor :type Actor%20Object%20Reference) (OtherComp :type Primitive%20Component%20Object%20Reference) (OtherBodyIndex :type Integer) (bFromSweep :type Boolean) (SweepResult :type Hit%20Result%20Structure%20%28by%20ref%29))
  (if (or (Variables|Default|GetBounce%20Enabled) (Variables|Default|GetHas%20Arrow))
    (CallFunction|Bounce OtherActor)))

(event OnComponentBeginOverlap(BottomSurface)
  (params (OverlappedComponent :type Primitive%20Component%20Object%20Reference) (OtherActor :type Actor%20Object%20Reference) (OtherComp :type Primitive%20Component%20Object%20Reference) (OtherBodyIndex :type Integer) (bFromSweep :type Boolean) (SweepResult :type Hit%20Result%20Structure%20%28by%20ref%29))
  (Utilities|Casting|CastToCrash_BP OtherActor)
  (CallFunction|BounceAction))

(event OnComponentEndOverlap(BottomSurface)
  (params (OverlappedComponent :type Primitive%20Component%20Object%20Reference) (OtherActor :type Actor%20Object%20Reference) (OtherComp :type Primitive%20Component%20Object%20Reference) (OtherBodyIndex :type Integer))
  (if (Variables|Default|GetPhysics%20Enabled)
    (Physics|SetSimulatePhysics (Variables|Components|GetStaticMesh) true)
    (Physics|AddImpulse (Variables|Components|GetStaticMesh) "0.000000,0.000000,500.000000" "None" true)))

(event Custom|Bounce%20Action)

(event Custom|Bounce%20Animation)

(fn ConstructionScript
  (Rendering|SetVisibility (Variables|Components|GetArrows) (Variables|Default|GetHas%20Arrow) true)
  (Rendering|Components|TextRender|SetText (Variables|Components|GetText1) (Variables|Default|GetBox%20Text)))

(fn Bounce
  (params (Overlapping%20Object :type Object%20Object%20Reference))
  (bind _ascrash_bp (Utilities|Casting|CastToCrash_BP Overlapping%20Object)
    (:then
      (Character|LaunchCharacter _ascrash_bp (* (Math|Vector|GetUpVector (Variables|Components|GetTop%20Surface)) (Math|Float|SelectFloat (Variables|Default|GetExtra%20Bounce%20Strenght) (Variables|Default|GetBounce%20Strenght) (Variables|Default|GetHas%20Arrow))) false true)
      (CallFunction|BounceAnimation)
      (CallFunction|BounceAction))
    (:CastFailed
      (if (Variables|Default|GetHas%20Arrow)
        (bind _asbox_base_bp (Utilities|Casting|CastToBox_Base_BP Overlapping%20Object))
        (Physics|SetPhysicsLinearVelocity (Variables|Box_Base_BP_C|GetStaticMesh _asbox_base_bp) "0.000000,0.000000,400.000000" false "None")))))