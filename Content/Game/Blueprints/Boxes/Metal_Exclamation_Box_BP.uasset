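; Metal exclamation box that acts as a switch, calling ActivateBoxes when triggered.
; A bottom-surface overlap, a bounce action or any damage all run the same path, which also disables bouncing.
; A timeline then slides the four text components outward along their forward vectors and hides TextRender, propagating to its children, when finished.
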(event OnComponentBeginOverlap(BottomSurface)
  (params (OverlappedComponent :type Primitive%20Component%20Object%20Reference) (OtherActor :type Actor%20Object%20Reference) (OtherComp :type Primitive%20Component%20Object%20Reference) (OtherBodyIndex :type Integer) (bFromSweep :type Boolean) (SweepResult :type Hit%20Result%20Structure%20%28by%20ref%29))
  (bind _text1 (Variables|Default|GetText1))
  (bind _text2 (Variables|Default|GetText2))
  (bind _text3 (Variables|Default|GetText3))
  (bind _text4 (Variables|Default|GetText4))
  (Variables|Default|SetBounce%20Enabled false)
  (Default|CallActivateBoxes)
  (bind _float (Timeline|Timeline_0 Play)
    (:Update
      (Utilities|FlowControl|Sequence
        (:then_0
          (Transformation|SetRelativeLocation _text1 (* (Math|Vector|GetForwardVector _text1) (Math|Float|Lerp 55.0 1e+02 _float)) false false))
        (:then_1
          (Transformation|SetRelativeLocation _text2 (* (Math|Vector|GetForwardVector _text2) (Math|Float|Lerp 55.0 1e+02 _float)) false false))
        (:then_2
          (Transformation|SetRelativeLocation _text3 (* (Math|Vector|GetForwardVector _text3) (Math|Float|Lerp 55.0 1e+02 _float)) false false))
        (:then_3
          (Transformation|SetRelativeLocation _text4 (* (Math|Vector|GetForwardVector _text4) (Math|Float|Lerp 55.0 1e+02 _float)) false false))))
    (:Finished
      (Rendering|SetVisibility (Variables|Default|GetTextRender) false true))))

(event EventBeginPlay
  (|CallParentFunction) ; This node is disabled and will not be called.\nDrag off pins to build functionality.
)

(event Collision|EventActorBeginOverlap
  (params (OtherActor :type Actor%20Object%20Reference))
  (|CallParentFunction OtherActor) ; This node is disabled and will not be called.\nDrag off pins to build functionality.
)

(event EventTick
  (params (DeltaSeconds :type Float%20%28single-precision%29))
  (|CallParentFunction DeltaSeconds) ; This node is disabled and will not be called.\nDrag off pins to build functionality.
)

(event EventBounceAction
  (bind _text1 (Variables|Default|GetText1))
  (bind _text2 (Variables|Default|GetText2))
  (bind _text3 (Variables|Default|GetText3))
  (bind _text4 (Variables|Default|GetText4))
  (Variables|Default|SetBounce%20Enabled false)
  (Default|CallActivateBoxes)
  (bind _float (Timeline|Timeline_0 Play)
    (:Update
      (Utilities|FlowControl|Sequence
        (:then_0
          (Transformation|SetRelativeLocation _text1 (* (Math|Vector|GetForwardVector _text1) (Math|Float|Lerp 55.0 1e+02 _float)) false false))
        (:then_1
          (Transformation|SetRelativeLocation _text2 (* (Math|Vector|GetForwardVector _text2) (Math|Float|Lerp 55.0 1e+02 _float)) false false))
        (:then_2
          (Transformation|SetRelativeLocation _text3 (* (Math|Vector|GetForwardVector _text3) (Math|Float|Lerp 55.0 1e+02 _float)) false false))
        (:then_3
          (Transformation|SetRelativeLocation _text4 (* (Math|Vector|GetForwardVector _text4) (Math|Float|Lerp 55.0 1e+02 _float)) false false))))
    (:Finished
      (Rendering|SetVisibility (Variables|Default|GetTextRender) false true))))

(event Game|Damage|EventAnyDamage
  (params (Damage :type Float%20%28single-precision%29) (DamageType :type Damage%20Type%20Object%20Reference) (InstigatedBy :type Controller%20Object%20Reference) (DamageCauser :type Actor%20Object%20Reference))
  (bind _text1 (Variables|Default|GetText1))
  (bind _text2 (Variables|Default|GetText2))
  (bind _text3 (Variables|Default|GetText3))
  (bind _text4 (Variables|Default|GetText4))
  (Variables|Default|SetBounce%20Enabled false)
  (Default|CallActivateBoxes)
  (bind _float (Timeline|Timeline_0 Play)
    (:Update
      (Utilities|FlowControl|Sequence
        (:then_0
          (Transformation|SetRelativeLocation _text1 (* (Math|Vector|GetForwardVector _text1) (Math|Float|Lerp 55.0 1e+02 _float)) false false))
        (:then_1
          (Transformation|SetRelativeLocation _text2 (* (Math|Vector|GetForwardVector _text2) (Math|Float|Lerp 55.0 1e+02 _float)) false false))
        (:then_2
          (Transformation|SetRelativeLocation _text3 (* (Math|Vector|GetForwardVector _text3) (Math|Float|Lerp 55.0 1e+02 _float)) false false))
        (:then_3
          (Transformation|SetRelativeLocation _text4 (* (Math|Vector|GetForwardVector _text4) (Math|Float|Lerp 55.0 1e+02 _float)) false false))))
    (:Finished
      (Rendering|SetVisibility (Variables|Default|GetTextRender) false true))))

(fn ConstructionScript
  (|CallParentFunction))