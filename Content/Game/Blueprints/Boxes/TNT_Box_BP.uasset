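; TNT box Blueprint that starts a timed countdown on a bounce action and explodes when it ends or when it takes any damage.
; BounceAction disables further bouncing and updates four text components through one-second delays before calling Explode.
; Explode switches the mesh to physics-only collision, applies full radial damage nearby, plays effect and sound, then calls Break.
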(event Custom|Explode
  (bind _returnvalue (Transformation|GetActorLocation))
  (Collision|SetCollisionEnabled (Variables|Default|GetStaticMesh) "PhysicsOnly")
  (Game|Damage|ApplyRadialDamage 1.0 (Transformation|GetWorldLocation (Variables|Default|GetStaticMesh)) 8e+01 0 0 self 0 true "ECC_GameTraceChannel1")
  (Effects|SpawnEmitteratLocation "/Game/StarterContent/Particles/P_Explosion.P_Explosion" _returnvalue)
  (Audio|PlaySoundatLocation "/Game/StarterContent/Audio/Explosion01.Explosion01" _returnvalue "0, 0, 0" 1.0 1.0 0.0 0 0 0 0)
  (CallFunction|Break))

(event EventBeginPlay
  (|CallParentFunction) ; This node is disabled and will not be called.\nDrag off pins to build functionality.
)

(event Collision|EventActorBeginOverlap
  (params (OtherActor :type Actor%20Object%20Reference))
  (|CallParentFunction OtherActor) ; This node is disabled and will not be called.\nDrag off pins to build functionality.
)

(event EventTick
  (params (DeltaSeconds :type Float%20%28single-precision%29))
  (|CallParentFunction DeltaSeconds) ; This node is disabled and will not be called.\nDrag off pins to build functionality.
)

(event Game|Damage|EventAnyDamage
  (params (Damage :type Float%20%28single-precision%29) (DamageType :type Damage%20Type%20Object%20Reference) (InstigatedBy :type Controller%20Object%20Reference) (DamageCauser :type Actor%20Object%20Reference))
  (CallFunction|Explode))

(event EventBounceAction
  (Variables|Default|SetBounce%20Enabled false)
  (Rendering|Components|TextRender|SetText (Variables|Default|GetText1) (Utilities|Text|ToText(Integer) (Variables|Default|GetSeconds)))
  (Utilities|FlowControl|Delay 1.0)
  (CallFunction|SetTNTText)
  (Utilities|FlowControl|Delay 1.0)
  (CallFunction|SetTNTText)
  (Utilities|FlowControl|Delay 1.0)
  (CallFunction|Explode))

(fn ConstructionScript
  (|CallParentFunction))

(fn SetTNTText
  (bind _result (Math|Integer|DecrementInt (Variables|Default|GetSeconds))
    (:%20%20
      (Rendering|Components|TextRender|SetText (Variables|Default|GetText1) (Utilities|Text|ToText(Integer) _result)))))